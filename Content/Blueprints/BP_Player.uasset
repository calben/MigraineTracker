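; Player Blueprint for inspecting brain parts with a visible mouse cursor, rotating its root by axis input with pitch clamped on vertical input.
; Primary click clears widgets, traces under the cursor and opens a WBP_SetMaterialValue widget for any BP_BrainPart hit.
; SwitchLookTarget moves a material gradient highlight between parts but is not called here.
; Tick performs the same trace and cast without acting on the result.
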(event `self.ReceiveBeginPlay`
  (set `PlayerController.bShowMouseCursor` true (`GameplayStatics.GetPlayerController` 0)))

(event `InputAxis|RotateRight`
  (params (AxisValue :type "Float (single-precision)"))
  (bind _defaultsceneroot (`self.DefaultSceneRoot`))
  (bind (_returnvalue_roll _returnvalue_pitch _returnvalue_yaw) (`KismetMathLibrary.BreakRotator` (`SceneComponent.K2_GetComponentRotation` _defaultsceneroot)))
  (`SceneComponent.K2_AddLocalRotation` (`self.DefaultSceneRoot`) (`KismetMathLibrary.MakeRotator` 0.0 0.0 AxisValue) false false)
  (`SceneComponent.K2_SetWorldRotation` _defaultsceneroot (`KismetMathLibrary.MakeRotator` 0.0 _returnvalue_pitch _returnvalue_yaw) false false))

(event `InputAxis|RotateUp`
  (params (AxisValue :type "Float (single-precision)"))
  (bind _defaultsceneroot (`self.DefaultSceneRoot`))
  (bind (_returnvalue_roll _returnvalue_pitch _returnvalue_yaw) (`KismetMathLibrary.BreakRotator` (`SceneComponent.K2_GetComponentRotation` _defaultsceneroot)))
  (`SceneComponent.K2_AddLocalRotation` _defaultsceneroot (`KismetMathLibrary.MakeRotator` 0.0 AxisValue) false false)
  (`SceneComponent.K2_SetWorldRotation` _defaultsceneroot (`KismetMathLibrary.MakeRotator` _returnvalue_roll (`KismetMathLibrary.ClampAngle` _returnvalue_pitch -30.0 30.0) _returnvalue_yaw) false false))

(event `InputAction|Primary`
  (params (Key :type "Key Structure"))
  (:`Pressed`
    (`WidgetLayoutLibrary.RemoveAllWidgets`)
    (bind _asbp_brain_part (cast `/Game/Blueprints/BP_BrainPart` (`.HitActor` (`GameplayStatics.BreakHitResult` (`PlayerController.GetHitResultUnderCursorByChannel` (`GameplayStatics.GetPlayerController` 0) "TraceTypeQuery1" true)))))
    (bind _returnvalue (`|CreateWidget` "/Game/UI/WBP_SetMaterialValue.WBP_SetMaterialValue_C"))
    (`/Game/UI/WBP_SetMaterialValue.Setup` _returnvalue _asbp_brain_part)
    (`UserWidget.AddToPlayerScreen` _returnvalue 0)))

(event `self.ReceiveTick`
  (params (DeltaSeconds :type "Float (single-precision)"))
  (cast `/Game/Blueprints/BP_BrainPart` (`.HitActor` (`GameplayStatics.BreakHitResult` (`PlayerController.GetHitResultUnderCursorByChannel` (`GameplayStatics.GetPlayerController` 0) "TraceTypeQuery1" true)))))

(fn `SwitchLookTarget`
  (params (InBrainPart :type "/Game/Blueprints/BP_BrainPart Object Reference"))
  (bind _looktarget (`self.LookTarget`))
  (bind _materialinstance (`/Game/Blueprints/BP_BrainPart.MaterialInstance` _looktarget))
  (`/Engine/EditorBlueprintResources/StandardMacros.IsValid` InBrainPart
    (:`Is Valid`
      (`|ExecutionSequence`
        (:`then_0`
          (`/Engine/EditorBlueprintResources/StandardMacros.IsValid` _looktarget
            (:`Is Valid`
              (`/Engine/EditorBlueprintResources/StandardMacros.IsValid` _materialinstance
                (:`Is Valid`
                  (`MaterialInstanceDynamic.SetScalarParameterValue` _materialinstance "GradientParameter" 0.0))))))
        (:`then_1`
          (bind _output_get (set `self.LookTarget` InBrainPart))
          (bind _materialinstance_2 (`/Game/Blueprints/BP_BrainPart.MaterialInstance` _output_get))
          (`/Engine/EditorBlueprintResources/StandardMacros.IsValid` _materialinstance_2
            (:`Is Valid`
              (`MaterialInstanceDynamic.SetScalarParameterValue` _materialinstance_2 "GradientParameter" 1.0))))))))

(fn `UserConstructionScript`)